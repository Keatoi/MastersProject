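; BP_T73 is a tank Blueprint that adds a screen UI when player-controlled and has a see-through body toggle.
; BeginPlay creates the WB_TankUi widget, and Tick projects the ScreenVector world location into that widget's ScreenPos.
; ScreenVector is only read in these graphs, never set.
; The 0 key uses a FlipFlop to swap the mesh's first material between transparent and regular T-72B body materials.
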(event `self.ReceiveBeginPlay`
  ;[1 1 1] Add UX to screen and set position if possessed
  (if (`self.IsPlayerControlled`)
    (bind _returnvalue (`|CreateWidget` "/Game/Blueprints/ChaosVehicle/WB_TankUi.WB_TankUi_C"))
    (bind _output_get (set `self.TankUI` _returnvalue))
    (`UserWidget.AddToViewport` _output_get 0)))

(event `self.ReceiveTick`
  (params (DeltaSeconds :type "Float (single-precision)"))
  ;[1 1 1] Add UX to screen and set position if possessed
  (if (`self.IsPlayerControlled`)
    (set `/Game/Blueprints/ChaosVehicle/WB_TankUi.ScreenPos` (`WidgetLayoutLibrary.ProjectWorldLocationToWidgetPosition` (`GameplayStatics.GetPlayerController` 0) (`self.ScreenVector`)) (`self.TankUI`))))

(event `Key|Zero`
  (params (Key :type "Key Structure"))
  (:`Pressed`
    (`/Engine/EditorBlueprintResources/StandardMacros.FlipFlop`
      (:`A`
        (`PrimitiveComponent.SetMaterial` (`self.Mesh`) 0 "/Game/Assets/Textures/Materials/M_East_Tank_T72b_BodyTransparent.M_East_Tank_T72b_BodyTransparent"))
      (:`B`
        (`PrimitiveComponent.SetMaterial` (`self.Mesh`) 0 "/Game/Assets/Textures/Materials/M_East_Tank_T72b_Body.M_East_Tank_T72b_Body")))))

(fn `UserConstructionScript`)