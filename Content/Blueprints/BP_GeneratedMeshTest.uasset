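; Test generated dynamic mesh actor that experiments with projectile-driven carving through Geometry Script.
; On rebuild it appends a box sized by dimension variables, applies PN tessellation, enables complex-as-simple collision and stores the result as TargetMesh.
; When a BP_BaseProjectile hits, it copies MeshRef into TargetMesh and uses that result as the tool for a boolean subtract on TargetMesh at the local-space hit point, then releases compute meshes.
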(event `self.OnRebuildGeneratedMesh`
  (params (TargetMesh :type "DynamicMesh Object Reference"))
  (bind _returnvalue (`GeometryScriptLibrary_MeshPrimitiveFunctions.AppendBox` TargetMesh (struct) (struct) (`self.Dimension X`) (`self.Dimension Y`) (`self.Dimension Z`) 0 0 0 "Base" null))
  (bind _returnvalue_2 (`GeometryScriptLibrary_MeshSubdivideFunctions.ApplyPNTessellation` _returnvalue (struct) 2 null))
  (`DynamicMeshComponent.EnableComplexAsSimpleCollision` (`self.DynamicMeshComponent`))
  (set `self.Target Mesh` _returnvalue_2)
  (`KismetSystemLibrary.PrintText` "Target Mesh Set" true true (struct :`G` 0.66 :`B` 1.0 :`A` 1.0) 20.0))

(event `self.DynamicMeshComponent.OnComponentHit`
  (params (HitComponent :type "PrimitiveComponent Object Reference") (OtherActor :type "Actor Object Reference") (OtherComp :type "PrimitiveComponent Object Reference") (NormalImpulse :type "Vector Structure") (Hit :type "HitResult Structure (by ref)"))
  (cast `/Game/Blueprints/Projectiles/BP_BaseProjectile` OtherActor)
  (`BaseDynamicMeshComponent.GetDynamicMesh` (`self.DynamicMeshComponent`))
  (bind _returnvalue (`GeometryScriptLibrary_StaticMeshFunctions.CopyMeshFromStaticMesh` (`self.MeshRef`) (`self.Target Mesh`) (struct) (struct) null)
    (:`Success`
      (`GeometryScriptLibrary_MeshBooleanFunctions.ApplyMeshBoolean` (`self.Target Mesh`) (struct) _returnvalue (`KismetMathLibrary.MakeTransform` (`KismetMathLibrary.InverseTransformLocation` (`SceneComponent.K2_GetComponentToWorld` (`self.DynamicMeshComponent`)) Hit_Location)) "Subtract" (struct) null)
      (`self.ReleaseAllComputeMeshes`))))

(fn `UserConstructionScript`)